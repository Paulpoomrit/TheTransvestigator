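; BP_Protagonist is the player character Blueprint, which links movement, animation, environment shaders and dialogue triggers.
; Each tick it writes its location to the PlayerLocation parameter of the MPC_Environment material parameter collection.
; Overlapping a BP_DialogueSpace calls that actor's Interact with the protagonist as argument.
; On jumping, it makes the animation component's instance jump straight to the Airborne node of the Locomotion state machine.
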(event `self.ReceiveActorBeginOverlap`
  (params (OtherActor :type "Actor Object Reference"))
  (`parent.ReceiveActorBeginOverlap` OtherActor)
  (bind _asbp_dialogue_space (cast `/Game/Dynamic/3_DialogueSystem/DialogueSpace/BP_DialogueSpace` OtherActor))
  (`/Game/Dynamic/3_DialogueSystem/BPI_Interactable.Interact` _asbp_dialogue_space self))

(event `self.ReceiveTick`
  (params (DeltaSeconds :type "Float (single-precision)"))
  (`parent.ReceiveTick` DeltaSeconds)
  (`KismetMaterialLibrary.SetVectorParameterValue` "/Game/Static/1_Shaders/1_EnvironmentMask/MPC_Environment.MPC_Environment" "PlayerLocation" (`KismetMathLibrary.Conv_VectorToLinearColor` (`self.K2_GetActorLocation`))))

(event `self.OnJumped`
  (`PaperZDAnimInstance.JumpToNode` (`PaperZDAnimationComponent.AnimInstance` (`self.AnimationComponent`)) "Airborne" "Locomotion"))

(fn `UserConstructionScript`
  (`parent.UserConstructionScript`))