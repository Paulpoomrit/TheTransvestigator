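; Dialogue component that scripts a press briefing in which the Spinmeister addresses a terrorist attack on an ally and fields a reporter's challenge.
; The Dialogue graph chains AddDialogue calls, branching on the returned state and option index.
; A three-way stance choice gives different replies, then rejoins a shared path that ends by calling StartSpinningComp after the reporter's accusation.
; AddDialogue and CloseConversation only forward to the parent class.
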(fn `AddDialogue`
  (params (Speaker :type Text) (Dialogue :type Text) (OptionText :type "Array of Text (by ref)"))
  (returns (State :type "/Game/Dynamic/3_DialogueSystem/E_DialogueState Enum") (OptionIndex :type Integer))
  (bind (_state _optionindex) (`parent.AddDialogue` Speaker Dialogue OptionText))
  (return _state _optionindex))

(fn `CloseConversation`
  (`parent.CloseConversation`))

(fn `Dialogue`
  (bind (_state _optionindex) (`self.AddDialogue` "Spinmeister" "Good morning. The recent terrorist attack has left our great ally deeply wounded and caused significant suffering and loss of life." (`|MakeArray` "CONTINUE" :!type "Text")))
  (switch `/Game/Dynamic/3_DialogueSystem/E_DialogueState` _state
    (:`NewEnumerator0`
      (switch `int` _optionindex
        (:`0`
          (bind (_state_2 _optionindex_2) (`self.AddDialogue` "Spinmeister" "The government’s stand on the conflict still remains the same; we stand...." (`|MakeArray` "With democracy." "With freedom of speech." "Stand by peace! " :!type "Text")))
          (switch `/Game/Dynamic/3_DialogueSystem/E_DialogueState` _state_2
            (:`NewEnumerator0`
              (switch `int` _optionindex_2
                (:`0`
                  (bind (_state_3 _optionindex_3) (`self.AddDialogue` "Spinmeister" "We stand with our ally, the only democratic nation in the Middle East. " (`|MakeArray` "CONTINUE" :!type "Text")))
                  (switch `/Game/Dynamic/3_DialogueSystem/E_DialogueState` _state_3
                    (:`NewEnumerator0`
                      (switch `int` _optionindex_3
                        (:`0`
                          _)))))
                (:`1`
                  (bind (_state_4 _optionindex_4) (`self.AddDialogue` "Spinmeister" "We stand with freedom of speech, freedom of expression, and human rights!" (`|MakeArray` "CONTINUE" :!type "Text")))
                  (switch `/Game/Dynamic/3_DialogueSystem/E_DialogueState` _state_4
                    (:`NewEnumerator0`
                      (switch `int` _optionindex_4
                        (:`0`
                          _)))))
                (:`2`
                  (bind (_state_5 _optionindex_5) (`self.AddDialogue` "Spinmeister" "We stand by peace! And condemn all unnecessary violence." (`|MakeArray` "CONTINUE" :!type "Text")))
                  (switch `/Game/Dynamic/3_DialogueSystem/E_DialogueState` _state_5
                    (:`NewEnumerator0`
                      (switch `int` _optionindex_5
                        (:`0`
                          _))))))
              (bind (_state_6 _optionindex_6) (`self.AddDialogue` "Spinmeister" "Any further questions are welcome." (`|MakeArray` "CONTINUE" :!type "Text")))
              (switch `/Game/Dynamic/3_DialogueSystem/E_DialogueState` _state_6
                (:`NewEnumerator0`
                  (switch `int` _optionindex_6
                    (:`0`
                      (bind (_state_7 _optionindex_7) (`self.AddDialogue` "News Reporter 1" "Sir, there are lots of complaints from people on the internet that what “our ally in the Middle East” is doing is essentially a continuation of colonialism." (`|MakeArray` "CONTINUE" :!type "Text")))
                      (switch `/Game/Dynamic/3_DialogueSystem/E_DialogueState` _state_7
                        (:`NewEnumerator0`
                          (switch `int` _optionindex_7
                            (:`0`
                              (bind (_state_8 _optionindex_8) (`self.AddDialogue` "News Reporter 1" "And what Amerika is doing is enabling and condoning them to do such a cruel project…" (`|MakeArray` "CONTINUE" :!type "Text")))
                              (switch `/Game/Dynamic/3_DialogueSystem/E_DialogueState` _state_8
                                (:`NewEnumerator0`
                                  (switch `int` _optionindex_8
                                    (:`0`
                                      (`self.StartSpinningComp`))))))))))))))))))))