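; Dialogue component for a news reporter, scripting a Host's broadcast about a terrorist attack in the Middle East and the government's response.
; The Dialogue function chains four AddDialogue calls, each offering one continue option and advancing on the Pass Through state with option index 0.
; After the handoff to a live Parliament Hill report it calls CloseConversation.
; AddDialogue and CloseConversation simply forward to the parent dialogue component.
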(fn `AddDialogue`
  (params (Speaker :type Text) (Dialogue :type Text) (OptionText :type "Array of Text (by ref)"))
  (returns (State :type "/Game/Dynamic/3_DialogueSystem/E_DialogueState Enum") (OptionIndex :type Integer))
  (bind (_state _optionindex) (`parent.AddDialogue` Speaker Dialogue OptionText))
  (return _state _optionindex))

(fn `CloseConversation`
  (`parent.CloseConversation`))

(fn `Dialogue`
  (bind (_state _optionindex) (`self.AddDialogue` "Host" "Thank you for joining us; this morning, a terrorist group attacked our great allies in the Middle East." (`|MakeArray` "CONTINUE" :!type "Text")))
  (switch `/Game/Dynamic/3_DialogueSystem/E_DialogueState` _state
    (:`NewEnumerator0`
      (switch `int` _optionindex
        (:`0`
          (bind (_state_2 _optionindex_2) (`self.AddDialogue` "Host" "This is the most devasting and perhaps most deadly attack in years. " (`|MakeArray` "Continue" :!type "Text")))
          (switch `/Game/Dynamic/3_DialogueSystem/E_DialogueState` _state_2
            (:`NewEnumerator0`
              (switch `int` _optionindex_2
                (:`0`
                  (bind (_state_3 _optionindex_3) (`self.AddDialogue` "Host" "“As the great nation of Amerika,” says the government’s spokesperson, “we’re prepared to help and alleviate all the pain as soon as possible.”" (`|MakeArray` "Continue" :!type "Text")))
                  (switch `/Game/Dynamic/3_DialogueSystem/E_DialogueState` _state_3
                    (:`NewEnumerator0`
                      (switch `int` _optionindex_3
                        (:`0`
                          (bind (_state_4 _optionindex_4) (`self.AddDialogue` "Host" "For more on America’s involvement in responding to this terrorist attack, let’s go live to Parliament Hill as the spokesperson is now preparing for a prompt response." (`|MakeArray` "Continue" :!type "Text")))
                          (switch `/Game/Dynamic/3_DialogueSystem/E_DialogueState` _state_4
                            (:`NewEnumerator0`
                              (switch `int` _optionindex_4
                                (:`0`
                                  (`self.CloseConversation`))))))))))))))))))