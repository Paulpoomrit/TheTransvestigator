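; Dialogue component scripting a press exchange in which News Reporter 3 challenges the Spinmeister over a land conflict.
; The Dialogue graph chains AddDialogue calls, branching on a three-option choice of scriptural replies.
; All branches rejoin at the reporter's ceasefire questions, which end by calling StartSpinningComp.
; AddDialogue and CloseConversation only forward to the parent component.
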(fn `AddDialogue`
  (params (Speaker :type Text) (Dialogue :type Text) (OptionText :type "Array of Text (by ref)"))
  (returns (State :type "/Game/Dynamic/3_DialogueSystem/E_DialogueState Enum") (OptionIndex :type Integer))
  (bind (_state _optionindex) (`parent.AddDialogue` Speaker Dialogue OptionText))
  (return _state _optionindex))

(fn `CloseConversation`
  (`parent.CloseConversation`))

(fn `Dialogue`
  (bind (_state _optionindex) (`self.AddDialogue` "News Reporter 3" "Sir, people are now questioning the very root of this conflict, the belief that the land was, indeed, “our land”…the holy land. " (`|MakeArray` "CONTINUE" :!type "Text")))
  (switch `/Game/Dynamic/3_DialogueSystem/E_DialogueState` _state
    (:`NewEnumerator0`
      (switch `int` _optionindex
        (:`0`
          (bind (_state_2 _optionindex_2) (`self.AddDialogue` "News Reporter 3" "It seems like the very need to create this “new state” started with the need to propel these people out of Europe, " (`|MakeArray` "CONTINUE" :!type "Text")))
          (switch `/Game/Dynamic/3_DialogueSystem/E_DialogueState` _state_2
            (:`NewEnumerator0`
              (switch `int` _optionindex_2
                (:`0`
                  (bind (_state_3 _optionindex_3) (`self.AddDialogue` "News Reporter 3" "it is, so they claimed, the Christian project of colonization and dispossession." (`|MakeArray` "CONTINUE" :!type "Text")))
                  (switch `/Game/Dynamic/3_DialogueSystem/E_DialogueState` _state_3
                    (:`NewEnumerator0`
                      (switch `int` _optionindex_3
                        (:`0`
                          (bind (_state_4 _optionindex_4) (`self.AddDialogue` "Spinmeister" "This is simply not true, as the scripture readily says that:" (`|MakeArray` "God already promised!" "They shall be God’s people" "God will take them." :!type "Text")))
                          (switch `/Game/Dynamic/3_DialogueSystem/E_DialogueState` _state_4
                            (:`NewEnumerator0`
                              (switch `int` _optionindex_4
                                (:`0`
                                  (bind (_state_5 _optionindex_5) (`self.AddDialogue` "Spinmeister" "God promised them a return to the holy land; they are the legitimate masters of Judea. " (`|MakeArray` "CONTINUE" :!type "Text")))
                                  (switch `/Game/Dynamic/3_DialogueSystem/E_DialogueState` _state_5
                                    (:`NewEnumerator0`
                                      (switch `int` _optionindex_5
                                        (:`0`
                                          _)))))
                                (:`1`
                                  (bind (_state_6 _optionindex_6) (`self.AddDialogue` "Spinmeister" "They shall be God’s people, and He will be their God; thus, He will assuredly plant them in this land, with all His heart, and with all His soul.”" (`|MakeArray` "CONTINUE" :!type "Text")))
                                  (switch `/Game/Dynamic/3_DialogueSystem/E_DialogueState` _state_6
                                    (:`NewEnumerator0`
                                      (switch `int` _optionindex_6
                                        (:`0`
                                          _)))))
                                (:`2`
                                  (bind (_state_7 _optionindex_7) (`self.AddDialogue` "Spinmeister" "God will take them from among the nations, gather them out of all countries, and bring them to this land. Then He will sprinkle clean water on them, and they shall be clean;" (`|MakeArray` "CONTINUE" :!type "Text")))
                                  (switch `/Game/Dynamic/3_DialogueSystem/E_DialogueState` _state_7
                                    (:`NewEnumerator0`
                                      (switch `int` _optionindex_7
                                        (:`0`
                                          _))))))
                              (bind (_state_8 _optionindex_8) (`self.AddDialogue` "News Reporter 3" "But, Sir, everyone now is calling for a ceasefire." (`|MakeArray` "CONTINUE" :!type "Text")))
                              (switch `/Game/Dynamic/3_DialogueSystem/E_DialogueState` _state_8
                                (:`NewEnumerator0`
                                  (switch `int` _optionindex_8
                                    (:`0`
                                      (bind (_state_9 _optionindex_9) (`self.AddDialogue` "News Reporter 3" "The government has promised a peace deal since day one, but our ally seems not to be interested in that at all." (`|MakeArray` "CONTINUE" :!type "Text")))
                                      (switch `/Game/Dynamic/3_DialogueSystem/E_DialogueState` _state_9
                                        (:`NewEnumerator0`
                                          (switch `int` _optionindex_9
                                            (:`0`
                                              (bind (_state_10 _optionindex_10) (`self.AddDialogue` "News Reporter 3" "When will we stop enabling such an atrocity to happen?" (`|MakeArray` "CONTINUE" :!type "Text")))
                                              (switch `/Game/Dynamic/3_DialogueSystem/E_DialogueState` _state_10
                                                (:`NewEnumerator0`
                                                  (switch `int` _optionindex_10
                                                    (:`0`
                                                      (`self.StartSpinningComp`))))))))))))))))))))))))))))